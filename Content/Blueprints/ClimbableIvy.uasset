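; Climbable ivy actor whose box volume lets the third-person character climb while overlapping it.
; Entering the box sets the character's walkable floor angle to vertical and turns on its IsClimbing flag.
; On exit, both are reset only if the character overlaps no other ClimbableIvy, so adjacent pieces work as one climbable area.
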(event `self.Box.OnComponentBeginOverlap`
  (params (OverlappedComponent :type "PrimitiveComponent Object Reference") (OtherActor :type "Actor Object Reference") (OtherComp :type "PrimitiveComponent Object Reference") (OtherBodyIndex :type Integer) (bFromSweep :type Boolean) (SweepResult :type "HitResult Structure (by ref)"))
  (bind _asthird_person_character (cast `/Game/PlayerCharacter/ThirdPersonCharacter` OtherActor))
  (`CharacterMovementComponent.SetWalkableFloorAngle` (`Character.CharacterMovement` _asthird_person_character) 90.0)
  (set `/Game/PlayerCharacter/ThirdPersonCharacter.bIsClimbing` true _asthird_person_character))

(event `self.Box.OnComponentEndOverlap`
  (params (OverlappedComponent :type "PrimitiveComponent Object Reference") (OtherActor :type "Actor Object Reference") (OtherComp :type "PrimitiveComponent Object Reference") (OtherBodyIndex :type Integer))
  (bind _asthird_person_character (cast `/Game/PlayerCharacter/ThirdPersonCharacter` OtherActor))
  (if (== (`KismetArrayLibrary.Array_Length` (`self.GetOverlappingActors` _asthird_person_character "ClimbableIvy_C")) 0)
    (`CharacterMovementComponent.SetWalkableFloorAngle` (`Character.CharacterMovement` _asthird_person_character) 44.765083)
    (set `/Game/PlayerCharacter/ThirdPersonCharacter.bIsClimbing` false _asthird_person_character)))

(fn `UserConstructionScript`)