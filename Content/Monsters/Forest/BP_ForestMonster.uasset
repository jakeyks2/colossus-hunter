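; Forest monster enemy that charges with its tusks and can only be hurt on bone "joint1" while stunned.
; While charging, Tick drives it forward and checks tusk overlaps: the player takes damage and ends the charge, while Landscape stuns the monster.
; A valid hit removes one health, then either ends the stun or marks it dead.
; UpdateDifficulty sets max health from the game instance, preserving damage already taken.
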(event `OnHit`
  (params (HitBone :type Name))
  (bind _charactermovement (`self.CharacterMovement`))
  (if (and (== HitBone "joint1") (`self.bIsStunned`))
    (`GameplayStatics.PlaySoundAtLocation` "/Game/Monsters/Forest/Sounds/ForestMonsterHurt.ForestMonsterHurt" (`self.K2_GetActorLocation`) (struct) 1.0 1.0 0.0 "/Game/Audio/SoundAttenuation.SoundAttenuation" null null)
    (bind _result (`/Engine/EditorBlueprintResources/StandardMacros.DecrementInt` (`self.Health`))
      (:`  `
        (if (> _result 0)
          (set `CharacterMovementComponent.bUseControllerDesiredRotation` true _charactermovement)
          (set `self.bIsStunned` false)
          (set `self.bIsCharging` false)
          (else
            (set `self.bIsDead` true)
            (set `CharacterMovementComponent.bUseControllerDesiredRotation` false _charactermovement)
            (set `self.bIsStunned` true)
            (set `self.bIsCharging` false)))))))

(event `self.ReceiveTick`
  (params (DeltaSeconds :type "Float (single-precision)"))
  (if (`self.bIsCharging`)
    (`self.AddMovementInput` (`self.GetActorForwardVector`))
    (for _array_element (`PrimitiveComponent.GetOverlappingActors` (`self.TuskCollider`) null)
      (bind _asthird_person_character (cast `/Game/PlayerCharacter/ThirdPersonCharacter` _array_element)
        (:`then`
          (bind _output_get (set `/Game/PlayerCharacter/ThirdPersonCharacter.Health` (- (stale _output_get) 60.0) _asthird_person_character))
          (`/Game/PlayerCharacter/ThirdPersonCharacter.UpdateHealth` _asthird_person_character)
          (set `CharacterMovementComponent.bUseControllerDesiredRotation` true (`self.CharacterMovement`))
          (set `self.bIsCharging` false))
        (:`CastFailed`
          (cast `Landscape` _array_element)
          (set `self.bIsStunned` true)
          (set `self.bIsCharging` false)))
      (`ActorComponent.Deactivate` (`self.RunningSound`)))))

(event `UpdateDifficulty`
  (bind _asthe_game_instance (cast `/Game/GameModes/TheGameInstance` (`GameplayStatics.GetGameInstance`)))
  (bind _returnvalue (select `int` (`/Game/GameModes/TheGameInstance.Difficulty` _asthe_game_instance) :`0` 2 :`1` 3 :`2` 4))
  (bind _output_get (set `self.Health` (+ (stale _output_get) (- _returnvalue (`self.MaxHealth`)))))
  (set `self.MaxHealth` _returnvalue))

(fn `UserConstructionScript`)