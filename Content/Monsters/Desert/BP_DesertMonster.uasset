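; BP_DesertMonster is a desert monster that burns the player with fire breath and is defeated through hits on specific bones.
; Tick drains health from a player inside the breath cone, or smoothly turns the monster toward its control rotation.
; Leg hits temporarily injure it and make its mesh walkable; Joint 3 hits remove health and launch the player away.
; Game-instance difficulty scales health, breath size, smoke duration and injury time.
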(event `self.ReceiveBeginPlay`
  (`self.UpdateDifficulty`))

(event `self.ReceiveTick`
  (params (DeltaSeconds :type "Float (single-precision)"))
  (bind (_returnvalue_roll _returnvalue_pitch _returnvalue_yaw) (`KismetMathLibrary.BreakRotator` (`self.GetControlRotation`)))
  (bind (_returnvalue_roll_2 _returnvalue_pitch_2 _returnvalue_yaw_2) (`KismetMathLibrary.BreakRotator` (`self.K2_GetActorRotation`)))
  (bind (_returnvalue_roll_3 _returnvalue_pitch_3 _returnvalue_yaw_3) (`KismetMathLibrary.BreakRotator` (`KismetMathLibrary.RInterpTo` (`KismetMathLibrary.MakeRotator` _returnvalue_roll_2 _returnvalue_pitch_2 _returnvalue_yaw_2) (`KismetMathLibrary.MakeRotator` _returnvalue_roll_2 _returnvalue_pitch_2 _returnvalue_yaw) (`GameplayStatics.GetWorldDeltaSeconds`) 4.0)))
  (if (`self.bIsFireSequenceActive`)
    (if (and (`self.bIsFireBreathActive`) (`self.bIsPlayerInCone`))
      (bind _asthird_person_character (cast `/Game/PlayerCharacter/ThirdPersonCharacter` (`GameplayStatics.GetPlayerPawn` 0)))
      (bind _output_get (set `/Game/PlayerCharacter/ThirdPersonCharacter.Health` (- (stale _output_get) (* DeltaSeconds 40.0)) _asthird_person_character))
      (`/Game/PlayerCharacter/ThirdPersonCharacter.UpdateHealth` _asthird_person_character))
    (elif (not (or (`self.bIsInjured`) (`self.bIsDead`)))
      (`self.K2_SetActorRotation` (`KismetMathLibrary.MakeRotator` _returnvalue_roll_3 _returnvalue_pitch_3 _returnvalue_yaw_3)))))

(event `self.Cone.OnComponentBeginOverlap`
  (params (OverlappedComponent :type "PrimitiveComponent Object Reference") (OtherActor :type "Actor Object Reference") (OtherComp :type "PrimitiveComponent Object Reference") (OtherBodyIndex :type Integer) (bFromSweep :type Boolean) (SweepResult :type "HitResult Structure (by ref)"))
  (cast `/Game/PlayerCharacter/ThirdPersonCharacter` OtherActor)
  (set `self.bIsPlayerInCone` true))

(event `self.Cone.OnComponentEndOverlap`
  (params (OverlappedComponent :type "PrimitiveComponent Object Reference") (OtherActor :type "Actor Object Reference") (OtherComp :type "PrimitiveComponent Object Reference") (OtherBodyIndex :type Integer))
  (cast `/Game/PlayerCharacter/ThirdPersonCharacter` OtherActor)
  (set `self.bIsPlayerInCone` false))

(event `OnHit`
  (params (HitBone :type Name))
  (bind _returnvalue (`GameplayStatics.GetPlayerPawn` 0))
  (bind _skeletalmesh (`self.SkeletalMesh`))
  (bind (_returnvalue_x _returnvalue_y) (`KismetMathLibrary.BreakVector` (* (`SceneComponent.GetRightVector` (`self.SkeletalMesh`)) -1500.0)))
  (switch `name` HitBone
    (:`joint6`
      (set `self.InjuredLeg` 6)
      (set `self.bIsInjured` true :!label _label)
      (`PrimitiveComponent.SetWalkableSlopeOverride` _skeletalmesh (make `WalkableSlopeOverride` "WalkableSlope_Increase" 90.0))
      (`KismetSystemLibrary.Delay` (`self.InjuredLength`))
      (set `self.bIsInjured` false)
      (`PrimitiveComponent.SetWalkableSlopeOverride` _skeletalmesh (make `WalkableSlopeOverride` "WalkableSlope_Default" 90.0))
      (if (<= (`self.GetDistanceTo` _returnvalue) 2000.0)
        (bind _asthird_person_character (cast `/Game/PlayerCharacter/ThirdPersonCharacter` _returnvalue))
        (`Character.LaunchCharacter` _asthird_person_character (`KismetMathLibrary.MakeVector` _returnvalue_x _returnvalue_y 1500.0) true true)))
    (:`joint13`
      (set `self.InjuredLeg` 13)
      (goto _label))
    (:`joint3`
      (`self.HitSequence`))))

(event `UpdateDifficulty`
  (bind _asthe_game_instance (cast `/Game/GameModes/TheGameInstance` (`GameplayStatics.GetGameInstance`)))
  (bind _difficulty (`/Game/GameModes/TheGameInstance.Difficulty` _asthe_game_instance))
  (bind _returnvalue (select `int` _difficulty :`0` 2 :`1` 3 :`2` 4))
  (bind _output_get (set `self.Health` (+ (stale _output_get) (- _returnvalue (`self.MaxHealth`)))))
  (set `self.MaxHealth` _returnvalue)
  (set `self.SmokeBreathDuration` (select `int` _difficulty :`0` 4.0 :`1` 2.0 :`2` 1.0 :!type "Float (single-precision)"))
  (`SceneComponent.SetRelativeScale3D` (`self.FireBreath`) (select `int` _difficulty :`0` (0.008 0.008 0.008) :`1` (0.01 0.01 0.01) :`2` (0.012 0.012 0.012) :!type "Vector Structure"))
  (`SceneComponent.SetRelativeScale3D` (`self.Cone`) (select `int` _difficulty :`0` (0.04 0.04 0.08) :`1` (0.05 0.05 0.1) :`2` (0.06 0.06 0.12) :!type "Vector Structure"))
  (set `self.InjuredLength` (select `int` _difficulty :`0` 30.0 :`1` 15.0 :`2` 10.0 :!type "Float (single-precision)")))

(fn `UserConstructionScript`)