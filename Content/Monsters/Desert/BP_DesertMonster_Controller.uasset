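; AI controller for the desert monster that runs its behavior tree and keeps its state in sync with the blackboard.
; On BeginPlay it focuses on the player pawn, and two seconds after possession it starts BT_DesertMonster.
; Every tick it copies the monster's IsInjured and IsDead flags into the blackboard for the tree to read.
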(event `self.ReceiveBeginPlay`
  (`self.K2_SetFocus` (`GameplayStatics.GetPlayerPawn` 0)))

(event `self.ReceivePossess`
  (params (PossessedPawn :type "Pawn Object Reference"))
  (`KismetSystemLibrary.Delay` 2.0)
  (`self.RunBehaviorTree` "/Game/Monsters/Desert/BT_DesertMonster.BT_DesertMonster"))

(event `self.ReceiveTick`
  (params (DeltaSeconds :type "Float (single-precision)"))
  (bind _blackboard (`self.Blackboard`))
  (`/Engine/EditorBlueprintResources/StandardMacros.IsValid` _blackboard
    (:`Is Valid`
      (bind _asbp_desert_monster (cast `/Game/Monsters/Desert/BP_DesertMonster` (`self.K2_GetPawn`)))
      (`BlackboardComponent.SetValueAsBool` _blackboard (`self.IsInjured`) (`/Game/Monsters/Desert/BP_DesertMonster.bIsInjured` _asbp_desert_monster))
      (`BlackboardComponent.SetValueAsBool` _blackboard (`self.IsDead`) (`/Game/Monsters/Desert/BP_DesertMonster.bIsDead` _asbp_desert_monster)))))

(fn `UserConstructionScript`)